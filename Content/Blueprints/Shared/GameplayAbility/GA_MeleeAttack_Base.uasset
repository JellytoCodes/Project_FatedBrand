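; Base melee attack gameplay ability, which turns the avatar toward its combat target and plays a random attack montage.
; It stores damage effect params from class defaults on the FatedBrand enemy as the montage starts, and ends when the montage finishes or is cut short.
; In parallel it waits for a successful-block event, then plays a block montage and ends after a short delay.
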(event Ability|EventActivateAbility
  (bind _returnvalue (Ability|GetAvatarActorfromActorInfo))
  (bind _returnvalue_2 (Class|CombatInterface|GetCombatTarget(Message) _returnvalue))
  (Class|CombatInterface|UpdateFacingTarget(Message) _returnvalue (Transformation|GetActorLocation _returnvalue_2))
  (Utilities|FlowControl|Sequence
    (:then_0
      (|PlayMontageandWaitProxy "None" (Utilities|Array|Get(acopy) (Variables|Default|GetAttackMontage) (Math|Random|RandomIntegerinRange 0 (- (Utilities|Array|Length (Variables|Default|GetAttackMontage)) 1))) 1.0 "None" true 1.0 0.0 false
        (:then
          (bind _returnvalue_3 (Class|FatedBrandGameplayAbility|MakeDamageEffectParamsfromClassDefaults 0))
          (Variables|/Script/Project_FatedBrand.FatedBrandCharacterBase|SetCombatDamageEffectParams (Class|FatedBrandGameplayAbility|GetFatedBrandEnemyfromActorInfo) _returnvalue_3))
        (:OnCompleted
          (Ability|EndAbility :!label _label))
        (:OnInterrupted
          (goto _label))
        (:OnCancelled
          (goto _label))))
    (:then_1
      (Ability|Tasks|WaitGameplayEvent "(TagName=\"Event.SuccessfulBlock\")" 0
        (:EventReceived
          (|PlayMontageandWaitProxy "None" "/Game/Blueprints/Enemy/MeleeAttacker_02/Animations/AM_Block.AM_Block" 1.0 "None" true 1.0 0.0 false
            (:OnCompleted
              _)
            (:OnInterrupted
              _)
            (:OnCancelled
              _))
          (Utilities|FlowControl|Delay 0.5)
          (Ability|EndAbility))))))
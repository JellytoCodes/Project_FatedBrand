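; Base Gameplay Ability for a ranged attack that fires a projectile at the avatar's combat target.
; On activation it captures the target's location, turns the avatar toward it through interface messages and plays a random attack montage.
; A gameplay event matching the configured tag triggers SpawnProjectile from a socket toward that saved location, so the aim does not track movement.
; The ability ends when the montage completes, is interrupted or is cancelled.
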(event Ability|EventActivateAbility
  (bind _returnvalue (Ability|GetAvatarActorfromActorInfo))
  (bind _returnvalue_2 (Class|CombatInterface|GetCombatTarget(Message) _returnvalue))
  (bind _output_get (Variables|Default|SetTargetLocation (Transformation|GetActorLocation _returnvalue_2)))
  (Class|CombatInterface|UpdateFacingTarget(Message) _returnvalue _output_get)
  (|PlayMontageandWaitProxy "None" (Utilities|Array|Get(acopy) (Variables|Default|GetAttackMontage) (Math|Random|RandomIntegerinRange 0 (- (Utilities|Array|Length (Variables|Default|GetAttackMontage)) 1))) 1.0 "None" true 1.0 0.0 false
    (:then
      (Ability|Tasks|WaitGameplayEvent (Variables|Default|GetEventTag) 0
        (:EventReceived
          (Class|FatedBrandProjectileAbility|SpawnProjectile (Variables|Default|GetTargetLocation) (Variables|Default|GetSocket%20Name) false (Variables|Default|GetPitch%20Override)))))
    (:OnCompleted
      (Ability|EndAbility :!label _label))
    (:OnInterrupted
      (goto _label))
    (:OnCancelled
      (goto _label))))
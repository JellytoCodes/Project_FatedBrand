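; BP_NextLevelActor is a level transition trigger that saves player progress and opens the main field map.
; When a CombatInterface actor overlaps its box, it disables box collision and the player's default mapping context, then fades the camera out.
; A Sequence saves the overlapping BP_FatedBrandCharacter's progress while the fade delay runs.
; After the delay, it holds the screen black and loads the level.
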(event OnComponentBeginOverlap(Box)
  (params (OverlappedComponent :type Primitive%20Component%20Object%20Reference) (OtherActor :type Actor%20Object%20Reference) (OtherComp :type Primitive%20Component%20Object%20Reference) (OtherBodyIndex :type Integer) (bFromSweep :type Boolean) (SweepResult :type Hit%20Result%20Structure%20%28by%20ref%29))
  (bind _returnvalue (Game|GetPlayerCameraManager 0))
  (bind _duration (Variables|Default|GetDuration))
  (bind _asbp_fated_brand_player_controller (Utilities|Casting|CastToBP_FatedBrandPlayerController (Game|GetPlayerController 0)))
  (if (Utilities|DoesObjectImplementInterface OtherActor "/Script/Project_FatedBrand.CombatInterface")
    (Utilities|FlowControl|Sequence
      (:then_0
        (Collision|SetCollisionEnabled (Variables|Default|GetBox) "NoCollision")
        (Class|FatedBrandPlayerController|DisableDefaultMappingContext _asbp_fated_brand_player_controller)
        (CameraFades|StartCameraFade :self _returnvalue :ToAlpha 2.0 :Duration _duration)
        (Utilities|FlowControl|Delay _duration)
        (Class|PlayerCameraManager|SetManualCameraFade :self _returnvalue :InFadeAmount 1.0)
        (Game|OpenLevel(byObjectReference) "/Game/Maps/MainFieldMap.MainFieldMap"))
      (:then_1
        (bind _asbp_fated_brand_character (Utilities|Casting|CastToBP_FatedBrandCharacter OtherActor))
        (Class|FatedBrandCharacter|SaveProgress _asbp_fated_brand_character (Utilities|Name|MakeLiteralName "None"))
        (Development|PrintString "Activate SavePoint")))))

(fn ConstructionScript)
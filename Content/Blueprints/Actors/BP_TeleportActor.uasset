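; BP_TeleportActor is a teleporter that moves combat-capable actors to its Scene component's location behind a screen fade.
; When an actor implementing CombatInterface stops overlapping the Box, it disables the player controller's default input mapping context and fades the camera out.
; After a delay it teleports that actor with zero rotation, fades back in, then re-enables input.
; Fade and input changes always target player 0, whichever actor triggered them.
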(event OnComponentEndOverlap(Box)
  (params (OverlappedComponent :type Primitive%20Component%20Object%20Reference) (OtherActor :type Actor%20Object%20Reference) (OtherComp :type Primitive%20Component%20Object%20Reference) (OtherBodyIndex :type Integer))
  (bind _returnvalue (Game|GetPlayerCameraManager 0))
  (bind _returnvalue_2 (Game|GetPlayerCameraManager 0))
  (bind _duration (Variables|Default|GetDuration))
  (bind _duration_2 (Variables|Default|GetDuration))
  (bind _asbp_fated_brand_player_controller (Utilities|Casting|CastToBP_FatedBrandPlayerController (Game|GetPlayerController 0)))
  (if (Utilities|DoesObjectImplementInterface OtherActor "/Script/Project_FatedBrand.CombatInterface")
    (Class|FatedBrandPlayerController|DisableDefaultMappingContext _asbp_fated_brand_player_controller)
    (CameraFades|StartCameraFade :self _returnvalue_2 :ToAlpha 2.0 :Duration _duration)
    (Utilities|FlowControl|Delay _duration)
    (Class|PlayerCameraManager|SetManualCameraFade :self _returnvalue_2 :InFadeAmount 1.0)
    (Transformation|Teleport OtherActor (Transformation|GetWorldLocation (Variables|Default|GetScene)) "0, 0, 0")
    (Utilities|FlowControl|Delay 0.2)
    (CameraFades|StartCameraFade :self _returnvalue :FromAlpha 1.0 :Duration _duration_2)
    (Utilities|FlowControl|Delay _duration_2)
    (Class|PlayerCameraManager|SetManualCameraFade :self _returnvalue)
    (Class|FatedBrandPlayerController|EnableDefaultMappingContext _asbp_fated_brand_player_controller)))

(fn ConstructionScript)
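; BP_GameEndActor is a trigger volume that ends the game when an actor implementing PlayerInterface overlaps its box.
; It hides that player's HUD message through the interface, then after a brief delay spawns a scaled Niagara portal effect offset from the player.
; A held camera fade starts with the effect, and the WBP_EndGame widget is added to the viewport after a further delay.
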(event OnComponentBeginOverlap(Box)
  (params (OverlappedComponent :type Primitive%20Component%20Object%20Reference) (OtherActor :type Actor%20Object%20Reference) (OtherComp :type Primitive%20Component%20Object%20Reference) (OtherBodyIndex :type Integer) (bFromSweep :type Boolean) (SweepResult :type Hit%20Result%20Structure%20%28by%20ref%29))
  (if (Utilities|DoesObjectImplementInterface OtherActor "/Script/Project_FatedBrand.PlayerInterface")
    (Variables|Default|SetOther%20Actor OtherActor)
    (Class|PlayerInterface|PlayerHideHUD(Message) (Variables|Default|GetOther%20Actor))
    (Utilities|FlowControl|Delay 0.2)
    (Niagara|SpawnSystematLocation "/Game/Assets/VFX/Sci-Fi_Starter_VFX_Pack_Niagara/Niagara/Portal/NS_Portal_2.NS_Portal_2" (+ (Transformation|GetActorLocation (Variables|Default|GetOther%20Actor)) "0.000000,60.000000,0.000000") "0, 0, 0" "2.000000,2.000000,2.000000")
    (CameraFades|StartCameraFade :self (Game|GetPlayerCameraManager 0) :ToAlpha 2.0 :Duration 5.0 :bHoldWhenFinished true)
    (Utilities|FlowControl|Delay 4.0)
    (bind _returnvalue (UserInterface|CreateWidget "/Game/Blueprints/UI/FadeInScreen/WBP_EndGame.WBP_EndGame_C"))
    (UserInterface|Viewport|AddtoViewport _returnvalue 0)))

(fn ConstructionScript)
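; BP_Rope is a swingable rope actor that characters can grab.
; A capsule overlap asks the other actor, via message calls, whether it can rope swing, then passes it the rope to grab.
; SwingForce pushes CableEnd with mass-independent acceleration scaled from swing input, only while the end hangs far enough below the actor origin, which stops pumping near the top of the arc.
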(event OnComponentBeginOverlap(Capsule)
  (params (OverlappedComponent :type Primitive%20Component%20Object%20Reference) (OtherActor :type Actor%20Object%20Reference) (OtherComp :type Primitive%20Component%20Object%20Reference) (OtherBodyIndex :type Integer) (bFromSweep :type Boolean) (SweepResult :type Hit%20Result%20Structure%20%28by%20ref%29))
  (bind _returnvalue (Class|PlayerInterface|CanRopeSwing(Message) OtherActor true))
  (if _returnvalue
    (Class|PlayerInterface|CanGrabRope(Message) OtherActor self)))

(event Custom|SwingForce
  (params (SwingInput :type Vector))
  (Variables|Default|SetSwing%20Input SwingInput)
  (if (not (< (- (.z (Transformation|GetActorLocation)) (.z (Transformation|GetWorldLocation (Variables|Default|GetCableEnd)))) 4.6e+02))
    (Physics|AddForce (Variables|Default|GetCableEnd) (* (Variables|Default|GetSwing%20Input) 2e+02) "None" true)))

(event EventBeginPlay)

(event Collision|EventActorBeginOverlap
  (params (OtherActor :type Actor%20Object%20Reference)))

(event EventTick
  (params (DeltaSeconds :type Float%20%28single-precision%29)))

(fn ConstructionScript)
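; BP_Vine is an effect actor that works as a periodically activating vine hazard or trigger.
; A looping timer set on BeginPlay repeatedly activates the Niagara effect and enables the box collision, then disables the collision after a set duration.
; Actors that begin overlapping the box are passed to OnBeginOverlap, whose logic is not defined in this graph.
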(event OnComponentBeginOverlap(Box)
  (params (OverlappedComponent :type Primitive%20Component%20Object%20Reference) (OtherActor :type Actor%20Object%20Reference) (OtherComp :type Primitive%20Component%20Object%20Reference) (OtherBodyIndex :type Integer) (bFromSweep :type Boolean) (SweepResult :type Hit%20Result%20Structure%20%28by%20ref%29))
  (Class|FatedBrandEffectActor|OnBeginOverlap OtherActor))

(event Custom|CustomEvent
  (Collision|SetCollisionEnabled (Variables|Default|GetBox) "QueryAndPhysics")
  (Components|Activation|Activate (Variables|Default|GetEffectNiagara) true)
  (Utilities|FlowControl|Delay (Variables|Default|GetCollisionEnabledDuration))
  (Collision|SetCollisionEnabled (Variables|Default|GetBox) "NoCollision"))

(event EventBeginPlay
  (Utilities|Time|SetTimerbyEvent (delegate Custom|CustomEvent) (Variables|Default|GetActiveLoopingTime) true))

(fn ConstructionScript)
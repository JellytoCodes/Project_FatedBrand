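; BP_TutorialMessageActor is a one-time tutorial prompt that fades in when the player character walks into its trigger box.
; On BeginPlay it creates a WBP_TutorialMessage widget, fills it with InfoScript text, assigns it to the InformationScreen widget component and hides the text.
; Box overlaps with BP_FatedBrandCharacter drive two timelines on the text's render opacity.
; Leaving the box plays DisableVisiblilty, then destroys the actor when it finishes.
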(event OnComponentBeginOverlap(Box)
  (params (OverlappedComponent :type Primitive%20Component%20Object%20Reference) (OtherActor :type Actor%20Object%20Reference) (OtherComp :type Primitive%20Component%20Object%20Reference) (OtherBodyIndex :type Integer) (bFromSweep :type Boolean) (SweepResult :type Hit%20Result%20Structure%20%28by%20ref%29))
  (Utilities|Casting|CastToBP_FatedBrandCharacter OtherActor)
  (bind _visibleopacity (Timeline|EnableVisiblilty Play)
    (:Update
      (Widget|SetRenderOpacity (Variables|/Game/Blueprints/UI/TutorialMessage/WBP_TutorialMessage.WBP_TutorialMessage_C|GetInfoMessage_Text (Variables|Default|GetTutorialWidget)) _visibleopacity))))

(event OnComponentEndOverlap(Box)
  (params (OverlappedComponent :type Primitive%20Component%20Object%20Reference) (OtherActor :type Actor%20Object%20Reference) (OtherComp :type Primitive%20Component%20Object%20Reference) (OtherBodyIndex :type Integer))
  (Utilities|Casting|CastToBP_FatedBrandCharacter OtherActor)
  (bind _visibleopacity (Timeline|DisableVisiblilty Play)
    (:Update
      (Widget|SetRenderOpacity (Variables|/Game/Blueprints/UI/TutorialMessage/WBP_TutorialMessage.WBP_TutorialMessage_C|GetInfoMessage_Text (Variables|Default|GetTutorialWidget)) _visibleopacity))
    (:Finished
      (Actor|DestroyActor))))

(event EventBeginPlay
  (bind _returnvalue (UserInterface|CreateWidget "/Game/Blueprints/UI/TutorialMessage/WBP_TutorialMessage.WBP_TutorialMessage_C"))
  (bind _output_get (Variables|Default|SetTutorialWidget _returnvalue))
  (Rendering|Components|TextRender|SetText (Variables|/Game/Blueprints/UI/TutorialMessage/WBP_TutorialMessage.WBP_TutorialMessage_C|GetInfoMessage_Text _output_get) (Variables|Default|GetInfoScript))
  (UserInterface|SetWidget (Variables|Default|GetInformationScreen) (Variables|Default|GetTutorialWidget))
  (Widget|SetRenderOpacity (Variables|/Game/Blueprints/UI/TutorialMessage/WBP_TutorialMessage.WBP_TutorialMessage_C|GetInfoMessage_Text (Variables|Default|GetTutorialWidget)) 0.0))

(fn ConstructionScript)
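; Gameplay ability for the first map boss's jump attack, a leap ending in an area-damage landing.
; It turns the boss toward its combat target and plays a fall montage while teleporting it forward and upward by set offsets.
; When that completes, a landing montage plays and a gameplay event triggers damage to live players within a radius around the boss.
; The ability ends when the landing montage completes, is interrupted or is cancelled.
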(event Custom|Land%20Attack%20Event
  (bind _returnvalue (Ability|GetAvatarActorfromActorInfo))
  (|PlayMontageandWaitProxy "None" "/Game/Blueprints/Enemy/FirstMapBoss/Animations/AM_JumpAttack_Land.AM_JumpAttack_Land" 1.0 "None" true 1.0 0.0 false
    (:then
      (Ability|Tasks|WaitGameplayEvent (Variables|Default|GetEvent%20Tag) 0
        (:EventReceived
          (bind _outoverlappingactors (Class|FatedBrandFunctionLibrary|GetLivePlayersWithinCircle _returnvalue (Utilities|Array|MakeArray _returnvalue) (Variables|Default|GetRadialDamageOuterRadius) (Transformation|GetActorLocation _returnvalue)))
          (for _array_element _outoverlappingactors
            (Class|FatedBrandGameplayAbility|CauseDamage _array_element)))))
    (:OnCompleted
      (Ability|EndAbility :!label _label))
    (:OnInterrupted
      (goto _label))
    (:OnCancelled
      (goto _label))))

(event Ability|EventActivateAbility
  (bind _returnvalue (Ability|GetAvatarActorfromActorInfo))
  (bind _returnvalue_2 (Class|CombatInterface|GetCombatTarget(Message) _returnvalue))
  (Class|CombatInterface|UpdateFacingTarget(Message) _returnvalue (Transformation|GetActorLocation _returnvalue_2))
  (|PlayMontageandWaitProxy "None" "/Game/Blueprints/Enemy/FirstMapBoss/Animations/AM_JumpAttack_Fall.AM_JumpAttack_Fall" 1.0 "None" true 1.0 0.0 false
    (:then
      (bind _jumploc (CallFunction|GetActorJumpLocation :!label _label))
      (Transformation|SetActorLocation (Ability|GetAvatarActorfromActorInfo) _jumploc false true))
    (:OnCompleted
      (CallFunction|LandAttackEvent))
    (:OnBlendedIn
      (goto _label))))

(fn GetActorJumpLocation
  (bind _returnvalue (Ability|GetAvatarActorfromActorInfo))
  (return (+ (Transformation|GetActorLocation _returnvalue) (* (Transformation|GetActorForwardVector _returnvalue) (Variables|Default|GetForwardVectorDist)) (* (Transformation|GetActorUpVector _returnvalue) (Variables|Default|GetUpVectorDist)))))
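; Base enemy Blueprint that handles death presentation, keeps the actor on the Y=0 plane and supports motion-warped facing.
; On death it disables capsule collision and starts the death montage alongside a timeline that drives a material FadeOut and shifts height, then destroys the actor.
; Animations pause on montage blend-out to hold the pose.
; Tick corrects Y drift, and UpdateFacingTarget sets the FacingTarget warp location.
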(event Custom|OnDeathDelegate_Event
  (params (DeadActor :type Actor%20Object%20Reference))
  (bind _returnvalue (Transformation|GetActorLocation))
  ;[1 1 1] Bind Delegate
  (Collision|SetCollisionEnabled (Variables|Default|GetCapsuleComponent) "NoCollision")
  (Animation|Montage|PlayMontage (Variables|Character|GetMesh) (Variables|Default|GetDeathMontage)
    (:then
      (bind _newtrack_0 (Timeline|Timeline PlayFromStart)
        (:Update
          (Rendering|Material|SetScalarParameterValueonMaterials (Variables|Character|GetMesh) "FadeOut" _newtrack_0)
          (Transformation|SetActorLocation (Math|Vector|MakeVector (.x _returnvalue) 0.0 (+ (.z _returnvalue) (* _newtrack_0 2.0))) false false))
        (:Finished
          (Actor|DestroyActor))))
    (:OnBlendOut
      (Variables|/Script/Engine.SkeletalMeshComponent|SetbPauseAnims (Variables|Character|GetMesh) true))))

(event EventBeginPlay
  ;[1 1 1] Bind Delegate
  (EventDispatchers|AssignOnDeathDelegate (delegate Custom|OnDeathDelegate_Event)))

(event EventUpdateFacingTarget
  (params (Target :type Vector%20%28by%20ref%29 :default "0, 0, 0"))
  ;[1 1 1] Update Facing
  (Class|MotionWarpingComponent|AddorUpdateWarpTargetfromLocation (Variables|Default|GetMotionWarpingComponent) "FacingTarget" Target))

(event EventTick
  (params (DeltaSeconds :type Float%20%28single-precision%29))
  (bind _returnvalue (Transformation|GetActorLocation))
  ;[1 0 0] Must Location Y = 0
  (if (!= (.y (Transformation|GetActorLocation)) 0.0)
    (Transformation|SetActorLocation (Math|Vector|MakeVector (.x _returnvalue) 0.0 (.z _returnvalue)) false false)))

(fn ConstructionScript)
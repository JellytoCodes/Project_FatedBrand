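; BP_RangeAttacker_01 is a ranged enemy Blueprint whose only active graph logic is a visual hit reaction.
; The HitReactAction event plays the HitReactEffect timeline, which drives the "Damage" scalar parameter on the mesh materials.
; BeginPlay, overlap and Tick are disabled stubs, and the construction script only calls its parent.
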(event EventBeginPlay
  (|CallParentFunction) ; This node is disabled and will not be called.\nDrag off pins to build functionality.
)

(event Collision|EventActorBeginOverlap
  (params (OtherActor :type Actor%20Object%20Reference))
  (|CallParentFunction OtherActor) ; This node is disabled and will not be called.\nDrag off pins to build functionality.
)

(event EventTick
  (params (DeltaSeconds :type Float%20%28single-precision%29))
  (|CallParentFunction DeltaSeconds) ; This node is disabled and will not be called.\nDrag off pins to build functionality.
)

(event EventHitReactAction
  (bind _newtrack_0 (Timeline|HitReactEffect Play)
    (:Update
      (Rendering|Material|SetScalarParameterValueonMaterials (Variables|Character|GetMesh) "Damage" _newtrack_0))))

(fn ConstructionScript
  (|CallParentFunction))
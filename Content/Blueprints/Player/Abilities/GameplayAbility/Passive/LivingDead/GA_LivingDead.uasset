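; GA_LivingDead is a passive player Gameplay Ability that gives a chance to revive instead of dying.
; On activation it commits, then rolls a random percentage against RevivalChance.
; Success starts a montage and immediately restores the avatar's health to a fixed value, ending the ability when the montage completes or is interrupted or cancelled.
; Failure calls PlayerDieMessage on the avatar and ends the ability.
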(event Ability|EventActivateAbility
  (bind _returnvalue (Ability|GetAvatarActorfromActorInfo))
  (Ability|CommitAbility)
  (if (< (Math|Random|RandomFloatinRange 1.0 1e+02) (Variables|Default|GetRevivalChance))
    (|PlayMontageandWaitProxy "None" "/Game/Characters/Animations/Ability/AM_Test.AM_Test" 1.0 "None" true 1.0 0.0 false
      (:then
        (Class|FatedBrandFunctionLibrary|SetCurrentHealth _returnvalue (Ability|GetAbilitySystemComponent _returnvalue) 5e+01))
      (:OnCompleted
        (Ability|EndAbility :!label _label))
      (:OnInterrupted
        (goto _label))
      (:OnCancelled
        (goto _label)))
    (else
      (Class|PlayerInterface|PlayerDie(Message) (Ability|GetAvatarActorfromActorInfo))
      (goto _label))))
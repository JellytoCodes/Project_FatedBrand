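; Player block ability that opens a very brief window to register a successful block.
; On activation it sends a gameplay event, starts a short timer that ends the ability, and waits for the SuccessfulBlock event.
; A successful block clears the timer, broadcasts weapon equipped, applies the VitalSurge charge effect to the player and plays the blocking montage.
; The ability ends when the montage finishes or is interrupted, broadcasting weapon unequipped.
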(event Custom|CustomEvent
  (Ability|EndAbility))

(event Ability|EventActivateAbility
  (bind _returnvalue (Class|FatedBrandGameplayAbility|GetFatedBrandAbilitySystemComponentfromActorInfo))
  (Utilities|FlowControl|Sequence
    (:then_0
      (Ability|SendGameplayEvent)
      (bind _returnvalue_2 (Utilities|Time|SetTimerbyEvent (delegate Custom|CustomEvent) 0.05))
      (Variables|Default|SetBlockingTimer _returnvalue_2))
    (:then_1
      (Ability|Tasks|WaitGameplayEvent "(TagName=\"Event.SuccessfulBlock\")" 0
        (:EventReceived
          (Utilities|Time|ClearandInvalidateTimerbyHandle (Variables|Default|GetBlockingTimer))
          (Class|FatedBrandCharacterBase|SendWeaponEquippedDelegate (Class|FatedBrandGameplayAbility|GetFatedBrandCharacterfromActorInfo) true)
          (GameplayEffects|ApplyGameplayEffectToSelf _returnvalue "/Game/Blueprints/Player/Abilities/GameplayEffect/GE_VitalSurge_Charge.GE_VitalSurge_Charge_C" 1.0 (GameplayEffects|MakeEffectContext _returnvalue))
          (|PlayMontageandWaitProxy "None" "/Game/Characters/Animations/MeleeAttack/AM_Blocking.AM_Blocking" 1.0 "None" true 1.0 0.0 false
            (:OnCompleted
              _)
            (:OnInterrupted
              _)
            (:OnCancelled
              _))
          (Ability|EndAbility))))))

(event Ability|EventOnEndAbility
  (params (bWasCancelled :type Boolean))
  (Class|FatedBrandCharacterBase|SendWeaponEquippedDelegate (Class|FatedBrandGameplayAbility|GetFatedBrandCharacterfromActorInfo) false))
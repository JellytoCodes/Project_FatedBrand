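; GA_NobleBlood is the Noble Blood player gameplay ability, an area damage attack centered on the avatar.
; On activation it commits, starts the AM_NobleBlood montage and immediately gathers live players within RadialDamageOuterRadius, excluding the avatar.
; Each player found takes damage and gets the GameplayCue.NobleBlood cue executed on their ability system component.
; The ability ends when the montage completes, is interrupted or is cancelled.
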(event Ability|EventActivateAbility
  (bind _returnvalue (Ability|GetAvatarActorfromActorInfo))
  (Ability|CommitAbility)
  (|PlayMontageandWaitProxy "None" "/Game/Characters/Retargeting/AM_NobleBlood.AM_NobleBlood" 1.0 "None" true 1.0 0.0 false
    (:then
      (bind _startloc (CallFunction|GetCharacterLocation))
      (bind _outoverlappingactors (Class|FatedBrandFunctionLibrary|GetLivePlayersWithinCircle _returnvalue (Utilities|Array|MakeArray _returnvalue) (Variables|Default|GetRadialDamageOuterRadius) _startloc))
      (for _array_element _outoverlappingactors
        (bind _returnvalue_2 (Class|FatedBrandGameplayAbility|CauseDamage _array_element))
        (Class|FatedBrandGameplayAbility|ExecuteGameplayCue (.TargetAbilitySystemComponent (Utilities|Struct|BreakDamageEffectParams _returnvalue_2)) (GameplayTags|MakeLiteralGameplayTag "(TagName=\"GameplayCue.NobleBlood\")"))))
    (:OnCompleted
      (Ability|EndAbility :!label _label))
    (:OnInterrupted
      (goto _label))
    (:OnCancelled
      (goto _label))))

(fn GetCharacterLocation
  (bind _returnvalue (Ability|GetAvatarActorfromActorInfo))
  (bind _returnvalue_2 (Transformation|GetActorLocation _returnvalue))
  (return _returnvalue_2 (+ _returnvalue_2 (Math|Vector|MakeVector (* (.x (Transformation|GetActorForwardVector _returnvalue)) (Variables|Default|GetRadialDamageOuterRadius)) 0.0 0.0))))
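; GA_VitalSurge is the player's Vital Surge gameplay ability, which only proceeds when the avatar's Vital Surge gauge meets a minimum threshold.
; It plays the Vital Surge montage while a WaitInputRelease task runs alongside, ending the ability if input is released.
; Montage blend-out applies the gauge spend effect to self before ending.
; Interruption, cancellation or an insufficient gauge ends it without applying that effect.
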(event Ability|EventActivateAbility
  (bind _returnvalue (Class|FatedBrandGameplayAbility|GetFatedBrandAbilitySystemComponentfromActorInfo))
  (bind _returnvalue_2 (Class|PlayerInterface|GetVitalSurgeGage(Message) (Ability|GetAvatarActorfromActorInfo)))
  (if (>= _returnvalue_2 3e+01)
    (Ability|Tasks|WaitInputRelease false
      (:then
        (|PlayMontageandWaitProxy "None" "/Game/Blueprints/Player/Animations/AM_VitalSurge.AM_VitalSurge" 1.0 "None" true 1.0 0.0 false
          (:OnBlendOut
            (GameplayEffects|ApplyGameplayEffectToSelf _returnvalue "/Game/Blueprints/Player/Abilities/GameplayEffect/GE_VitalSurge_Spend.GE_VitalSurge_Spend_C" 1.0 (GameplayEffects|MakeEffectContext _returnvalue)))
          (:OnInterrupted
            _)
          (:OnCancelled
            _))
        (Ability|EndAbility))
      (:OnRelease
        (Ability|EndAbility :!label _label)))
    (else
      (goto _label))))
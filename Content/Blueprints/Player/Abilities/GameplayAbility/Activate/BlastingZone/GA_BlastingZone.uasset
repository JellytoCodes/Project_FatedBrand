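; GA_BlastingZone is a player gameplay ability that performs the Blasting Zone attack through a montage.
; On activation it commits, signals weapon equipped and copies damage effect params from class defaults to the character's combat params.
; A melee montage event executes the BlastingZone gameplay cue on the target ability system component from those params.
; The ability ends when the montage completes, is interrupted or is cancelled, and OnEndAbility signals weapon unequipped.
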(event Ability|EventActivateAbility
  (Ability|CommitAbility)
  (Class|FatedBrandCharacterBase|SendWeaponEquippedDelegate (Class|FatedBrandGameplayAbility|GetFatedBrandCharacterfromActorInfo) true)
  (bind _returnvalue (Class|FatedBrandGameplayAbility|MakeDamageEffectParamsfromClassDefaults 0))
  (Variables|/Script/Project_FatedBrand.FatedBrandCharacterBase|SetCombatDamageEffectParams (Class|FatedBrandGameplayAbility|GetFatedBrandCharacterfromActorInfo) _returnvalue)
  (|PlayMontageandWaitProxy "None" "/Game/Characters/Retargeting/AM_BlastingZone.AM_BlastingZone" 1.0 "None" true 1.0 0.0 false
    (:then
      (Ability|Tasks|WaitGameplayEvent "(TagName=\"Event.Montage.Melee\")" 0
        (:EventReceived
          (Class|FatedBrandGameplayAbility|ExecuteGameplayCue (.TargetAbilitySystemComponent (Utilities|Struct|BreakDamageEffectParams (Variables|/Script/Project_FatedBrand.FatedBrandCharacterBase|GetCombatDamageEffectParams (Class|FatedBrandGameplayAbility|GetFatedBrandCharacterfromActorInfo)))) (GameplayTags|MakeLiteralGameplayTag "(TagName=\"GameplayCue.BlastingZone\")")))))
    (:OnCompleted
      (Ability|EndAbility :!label _label))
    (:OnInterrupted
      (goto _label))
    (:OnCancelled
      (goto _label))))

(event Ability|EventOnEndAbility
  (params (bWasCancelled :type Boolean))
  (Class|FatedBrandCharacterBase|SendWeaponEquippedDelegate (Class|FatedBrandGameplayAbility|GetFatedBrandCharacterfromActorInfo) false))
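; Melee attack gameplay ability that plays a looping montage combo for the FatedBrand character.
; Activation signals weapon equipped, cancels any pending combo reset and stores class-default damage effect params on the character.
; An input-press task plays the montage at the current combo index, which then advances and wraps.
; When the montage finishes or is interrupted, the ability ends and starts a short timer that resets the combo and signals weapon unequipped.
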(event Custom|ComboReset
  (Class|FatedBrandCharacterBase|SendWeaponEquippedDelegate (Class|FatedBrandGameplayAbility|GetFatedBrandCharacterfromActorInfo) false)
  (Variables|Default|SetLoopMontage 0))

(event Ability|EventActivateAbility
  (Utilities|FlowControl|Sequence
    (:then_0
      (Class|FatedBrandCharacterBase|SendWeaponEquippedDelegate (Class|FatedBrandGameplayAbility|GetFatedBrandCharacterfromActorInfo) true)
      (Utilities|Time|ClearandInvalidateTimerbyHandle (Variables|Default|GetComboResetTimer))
      (bind _returnvalue (Class|FatedBrandGameplayAbility|MakeDamageEffectParamsfromClassDefaults 0))
      (Variables|/Script/Project_FatedBrand.FatedBrandCharacterBase|SetCombatDamageEffectParams (Class|FatedBrandGameplayAbility|GetFatedBrandCharacterfromActorInfo) _returnvalue))
    (:then_1
      (Ability|Tasks|WaitInputPress true
        (:OnPress
          (|PlayMontageandWaitProxy "None" (Utilities|Array|Get(acopy) (Variables|Default|GetMontage%20to%20Play) (Variables|Default|GetLoopMontage)) 1.0 "None" true 1.0 0.0 false
            (:then
              (bind _result (Math|Integer|IncrementInt (Variables|Default|GetLoopMontage))
                (:%20%20
                  (if (>= _result 3)
                    (Variables|Default|SetLoopMontage 0)))))
            (:OnCompleted
              (Ability|EndAbility :!label _label)
              (bind _returnvalue_2 (Utilities|Time|SetTimerbyEvent (delegate Custom|ComboReset) 0.3))
              (Variables|Default|SetComboResetTimer _returnvalue_2))
            (:OnBlendOut
              (goto _label))
            (:OnInterrupted
              (goto _label))
            (:OnCancelled
              (goto _label))))))))